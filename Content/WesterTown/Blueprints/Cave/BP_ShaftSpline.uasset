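; BP_ShaftSpline is a construction-script tool that builds a cave mine shaft with carts along a spline.
; It lays collidable spline meshes at fixed spacing, with distinct meshes at each end and cycling tunnel variants between.
; A row of cart meshes follows the spline from an adjustable normalized position.
; All generation runs only when DisableForFasterEditing is true, despite that flag's name.
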(event EventBeginPlay)

(event Collision|EventActorBeginOverlap
  (params (OtherActor :type Actor%20Object%20Reference)))

(event EventTick
  (params (DeltaSeconds :type Float%20%28single-precision%29)))

(fn ConstructionScript
  (bind _spline (Variables|Default|GetSpline))
  (bind _spacing (Variables|Spline|GetSpacing))
  (bind _tangentscale (Variables|Spline|GetTangentScale))
  (bind _spline_2 (Variables|Default|GetSpline))
  (bind _returnvalue (Spline|GetSplineLength _spline))
  (bind _returnvalue_2 (Math|Float|Division(WholeandRemainder) _returnvalue _spacing))
  (if (Variables|Spline|GetDisableForFasterEditing)
    (for _index (range 0 _returnvalue_2)
      ;[1 1 1] Start and End Spline
      (bind _returnvalue_3 (AddComponent|AddSplineMeshComponent true))
      (Collision|SetCollisionEnabled _returnvalue_3 "QueryAndPhysics")
      (if (== _index 0)
        ;;[1 1 1] End Spline Mesh
        (Components|StaticMesh|SetStaticMesh _returnvalue_3 "/Game/WesterTown/Models/Nature/Cave/SM_Cave_Shaft_End1.SM_Cave_Shaft_End1")
        (elif (< _index _returnvalue_2)
          ;[1 1 1] In Between Spline
          (if (>= (Variables|Default|GetMeshNumber) (Utilities|Array|Length (Variables|Spline|GetTunnelMeshes)))
            (Variables|Default|SetMeshNumber 1)
            (else
              (Variables|Default|SetMeshNumber (+ 1 (Variables|Default|GetMeshNumber)))))
          (Components|StaticMesh|SetStaticMesh _returnvalue_3 (Utilities|Array|Get(acopy) (Variables|Spline|GetTunnelMeshes) (- (Variables|Default|GetMeshNumber) 1)))
          (else
            ;;[1 1 1] Start Spline Mesh
            (Components|StaticMesh|SetStaticMesh _returnvalue_3 "/Game/WesterTown/Models/Nature/Cave/SM_Cave_Shaft_Start1.SM_Cave_Shaft_Start1"))))
      (SplineMesh|SetStartandEnd _returnvalue_3 (Spline|GetLocationatDistanceAlongSpline _spline (* _index _spacing) "World") (* (Spline|GetDirectionatDistanceAlongSpline _spline (* _index _spacing) "World") _tangentscale) (Spline|GetLocationatDistanceAlongSpline _spline (+ (* _index _spacing) _spacing) "World") (* (Spline|GetDirectionatDistanceAlongSpline _spline (+ (* _index _spacing) _spacing) "World") _tangentscale) true :!class /Script/Engine.SplineMeshComponent))
    ;[1 1 1] Add Carts
    (for _index_2 (range 0 (- (Variables|Default|GetNumberOfCarts) 1))
      (bind _returnvalue_4 (AddComponent|AddStaticMeshComponent false))
      (Transformation|SetRelativeLocationAndRotation _returnvalue_4 (Spline|GetLocationatDistanceAlongSpline _spline_2 (+ (Math|Float|Lerp 0.0 (Spline|GetSplineLength _spline_2) (Variables|Default|GetCartPosition)) (* _index_2 (Variables|Default|GetCartSpacing))) "Local") (Spline|GetRotationatDistanceAlongSpline _spline_2 (+ (Math|Float|Lerp 0.0 (Spline|GetSplineLength _spline_2) (Variables|Default|GetCartPosition)) (* _index_2 (Variables|Default|GetCartSpacing))) "Local") false false))))